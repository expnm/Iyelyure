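; BP_Generator procedurally builds a layout of floor and wall actors on BeginPlay.
; It spawns a set number of Floor1 actors in a chain, querying each for its joints and picking a random joint as the next spawn point.
; After each floor is placed, it spawns a randomly chosen Wall1 or Wall2 at every joint of that floor, including the one picked for continuation.
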(event EventBeginPlay
  (for _index (range 1 (Variables|Default|GetFloor_1_Count))
    (bind _returnvalue (Game|SpawnActorfromClass (Variables|Default|GetFloor_1) (Variables|Default|GetSpawnPoint) "Undefined" "MultiplyWithRoot" 0 0))
    (bind _joints (Class|BIFloor|GetJoints(Message) _returnvalue))
    (Variables|Default|SetSpawnPoint (.position (.OutItem (Utilities|Array|Random _joints))))
    (for _array_element _joints
      (Game|SpawnActorfromClass (.OutItem (Utilities|Array|Random (Utilities|Array|MakeArray (Variables|Default|GetWall_1) (Variables|Default|GetWall_2)))) (.position _array_element) "Undefined" "MultiplyWithRoot" 0 0))))

(fn ConstructionScript)