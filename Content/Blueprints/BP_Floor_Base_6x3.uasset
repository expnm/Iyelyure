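; BP_Floor_Base_6x3 is a floor base piece that exposes six joint points, J1 to J6.
; GetJoints gathers each joint component's world transform into a result collection, leaving the second field of each entry unfilled.
; The event graph and construction script are empty, so this joint query is the only logic in the Blueprint.
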(event EventBeginPlay)

(event Collision|EventActorBeginOverlap
  (params (OtherActor :type Actor%20Object%20Reference)))

(event EventTick
  (params (DeltaSeconds :type Float%20%28single-precision%29)))

(fn ConstructionScript)

(fn GetJoints
  (bind _result (LocalVariables|GetResult))
  (Utilities|Array|Add _result (Utilities|Struct|MakeF_JointInfo (Transformation|GetWorldTransform (Variables|Default|GetJ1)) "NewEnumerator0"))
  (Utilities|Array|Add _result (Utilities|Struct|MakeF_JointInfo (Transformation|GetWorldTransform (Variables|Default|GetJ2)) "NewEnumerator0"))
  (Utilities|Array|Add _result (Utilities|Struct|MakeF_JointInfo (Transformation|GetWorldTransform (Variables|Default|GetJ3)) "NewEnumerator0"))
  (Utilities|Array|Add _result (Utilities|Struct|MakeF_JointInfo (Transformation|GetWorldTransform (Variables|Default|GetJ4)) "NewEnumerator0"))
  (Utilities|Array|Add _result (Utilities|Struct|MakeF_JointInfo (Transformation|GetWorldTransform (Variables|Default|GetJ5)) "NewEnumerator0"))
  (Utilities|Array|Add _result (Utilities|Struct|MakeF_JointInfo (Transformation|GetWorldTransform (Variables|Default|GetJ6)) "NewEnumerator0"))
  (return _result))